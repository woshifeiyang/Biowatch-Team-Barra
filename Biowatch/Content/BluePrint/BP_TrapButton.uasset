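; BP_TrapButton is a clickable in-world button that fires the currently selected trap.
; BeginPlay enables click events on the player controller so the Cylinder mesh receives OnClicked.
; A click lowers the cylinder, then reads CurrentTrap from the level's Camera_Tracker actor.
; A valid BP_Trap is triggered before the cylinder moves back; an invalid one prints a debug message.
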(event `self.ReceiveBeginPlay`
  (set `PlayerController.bEnableClickEvents` true (`GameplayStatics.GetPlayerController` 0)))

(event `self.Cylinder.OnClicked`
  (params (TouchedComponent :type "PrimitiveComponent Object Reference") (ButtonPressed :type "Key Structure"))
  (bind _cylinder (`self.Cylinder`))
  (`KismetSystemLibrary.MoveComponentTo` _cylinder (0.0 0.0 -50.0) (struct) false false 0.25)
  (bind _returnvalue (`GameplayStatics.GetActorOfClass` "/Game/BluePrint/Camera_Tracker.Camera_Tracker_C"))
  (bind _currenttrap (`/Game/BluePrint/Camera_Tracker.CurrentTrap` _returnvalue))
  (`/Engine/EditorBlueprintResources/StandardMacros.IsValid` _currenttrap
    (:`Is Valid`
      (bind _asbp_trap (cast `/Game/BluePrint/BP_Trap` _currenttrap))
      (`/Game/BluePrint/BP_Trap.Trigger` _asbp_trap)
      (`KismetSystemLibrary.MoveComponentTo` _cylinder (0.0 0.0 0.0) (struct) false false 0.25))
    (:`Is Not Valid`
      (`KismetSystemLibrary.PrintString` "CurrTrap is not Valid")
      (`KismetSystemLibrary.MoveComponentTo` null (0.0 0.0 0.0) (struct) false false 0.25))))

(fn `UserConstructionScript`)