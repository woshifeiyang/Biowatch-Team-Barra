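; BP_PipeStraight is a pipe actor built from spline meshes along its SplineWire spline, with no active gameplay logic.
; The construction script adds a manually attached, X-forward spline mesh component between each pair of neighbouring spline points.
; Segment positions and tangents are read in world space, and both start and end tangents come from the segment's end point.
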(fn `UserConstructionScript`
  (bind _splinewire (`self.SplineWire`))
  (for _index (range (+ (- (`SplineComponent.GetNumberOfSplinePoints` (`self.SplineWire`)) 2) 1))
    (bind _returnvalue (`AddComponent|NODE_AddSplineMeshComponent-0` :`bManualAttachment` true))
    (`SplineMeshComponent.SetForwardAxis` _returnvalue "X" true)
    (bind _returnvalue_2 (+ _index 1))
    (`SplineMeshComponent.SetStartAndEnd` _returnvalue (`SplineComponent.GetLocationAtSplinePoint` _splinewire _index "World") (`SplineComponent.GetTangentAtSplinePoint` _splinewire _returnvalue_2 "World") (`SplineComponent.GetLocationAtSplinePoint` _splinewire _returnvalue_2 "World") (`SplineComponent.GetTangentAtSplinePoint` _splinewire _returnvalue_2 "World") true)))