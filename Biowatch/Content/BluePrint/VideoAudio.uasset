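; VideoAudio is a Blueprint that controls video audio for the BioWatchSTV tutorial and full media sources, plus a toggle for level audio.
; Separate events open the tutorial cut or the full source on the MediaSound component's media player, and a skip event closes that player.
; The level audio toggle loops over an array of objects and flips the active state of each one's root component.
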(event `TutorialAudio`
  (`MediaPlayer.OpenSource` (`MediaSoundComponent.GetMediaPlayer` (`self.MediaSound`)) "/Game/Movies/BioWatchSTV_TUTORIALCUT.BioWatchSTV_TUTORIALCUT"))

(event `FullAudio`
  (`MediaPlayer.OpenSource` (`MediaSoundComponent.GetMediaPlayer` (`self.MediaSound`)) "/Game/Movies/BioWatchSTV_FULL.BioWatchSTV_FULL"))

(event `SkippedFULL`
  (`MediaPlayer.Close` (`MediaSoundComponent.GetMediaPlayer` (`self.MediaSound`))))

(event `ToggleLevelAudio`
  (for _array_element (`self.obejcts`)
    (`ActorComponent.ToggleActive` (`Actor.RootComponent` _array_element))))

(fn `UserConstructionScript`)