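; Incubation prison pod that drains its goo and hands off from the creature inside to the playable or level creature character.
; DrainPod activates the drain effect and opens a gate that lets Tick keep lowering the Goo component.
; After an optional delay it plays a fade-out sequence, destroys the pod's Creature component, starts up CreatureCharacter, notifies Camera_Tracker and closes the gate.
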(event `self.ReceiveTick`
  (params (DeltaSeconds :type "Float (single-precision)"))
  (bind _goo (`self.goo`))
  (bind (_relativelocation_x _relativelocation_y _relativelocation_z) (`KismetMathLibrary.BreakVector` (`SceneComponent.RelativeLocation` _goo)))
  (`/Engine/EditorBlueprintResources/StandardMacros.Gate` true :!label _label
    (:`Exit`
      (`KismetSystemLibrary.MoveComponentTo` _goo (`KismetMathLibrary.MakeVector` _relativelocation_x _relativelocation_y (+ _relativelocation_z -6.0))))))

(event `DrainPod`
  (`ActorComponent.Activate` (`self.GooDrain`) false)
  (`|ExecutionSequence`
    (:`then_0`
      (if (not (`self.skipDrain`))
        (`KismetSystemLibrary.Delay` 5.0))
      (bind (_outactor _returnvalue) (`LevelSequencePlayer.CreateLevelSequencePlayer` "/Game/FadeOut.FadeOut"))
      (`MovieSceneSequencePlayer.Play` _returnvalue)
      (`KismetSystemLibrary.Delay` 3.0)
      (`ActorComponent.K2_DestroyComponent` (`self.creature`))
      (`ActorComponent.Deactivate` (`self.GooDrain`))
      (bind _returnvalue_2 (`GameplayStatics.GetActorOfClass` "/Game/Creature/CreatureCharacter.CreatureCharacter_C"))
      (`/Game/Creature/CreatureCharacter.CreaturestartUp` _returnvalue_2)
      (bind _returnvalue_3 (`GameplayStatics.GetActorOfClass` "/Game/BluePrint/Camera_Tracker.Camera_Tracker_C"))
      (`/Game/BluePrint/Camera_Tracker.PodIsopen` _returnvalue_3)
      (goto _label :!via `Close`))
    (:`then_1`
      (goto _label :!via `Open`))))

(fn `UserConstructionScript`)