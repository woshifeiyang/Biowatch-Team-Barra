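; BP_PowerButton is a clickable button that drains an incubation prison pod and sets off alarms.
; BeginPlay enables click events, and each click plays the OfficeButton component, while a gate lets the main sequence fire only once.
; That sequence forces Camera_Tracker to cam 0, moves the Cylinder down, drains the referenced Pod and activates every BP_Alarm in the Alarms array.
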(event `self.ReceiveBeginPlay`
  (set `PlayerController.bEnableClickEvents` true (`GameplayStatics.GetPlayerController` 0)))

(event `self.ReceiveActorOnClicked`
  (params (ButtonPressed :type "Key Structure"))
  (`AudioComponent.Play` (`self.OfficeButton`) 0.0)
  (`/Engine/EditorBlueprintResources/StandardMacros.Gate` false :!label _label
    (:`Exit`
      (`|ExecutionSequence`
        (:`then_0`
          (bind _returnvalue (`GameplayStatics.GetActorOfClass` "/Game/BluePrint/Camera_Tracker.Camera_Tracker_C"))
          (`/Game/BluePrint/Camera_Tracker.ForceCam0` _returnvalue)
          (`KismetSystemLibrary.MoveComponentTo` (`self.Cylinder`) (0.0 0.0 -5.0) (struct) false false 0.25)
          (bind _asbp_incubation_prison (cast `/Game/Environment_Assets/BP_Incubation_prison` (`self.Pod`)))
          (`/Game/Environment_Assets/BP_Incubation_prison.DrainPod` _asbp_incubation_prison)
          (for _array_element (`self.Alarms`)
            (bind _asbp_alarm (cast `/Game/BluePrint/BP_Alarm` _array_element))
            (`/Game/BluePrint/BP_Alarm.Activate` _asbp_alarm)))
        (:`then_1`
          (goto _label :!via `Close`))))))

(fn `UserConstructionScript`)