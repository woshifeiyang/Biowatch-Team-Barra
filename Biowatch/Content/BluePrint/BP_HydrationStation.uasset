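; Hydration station Blueprint: a shower that sprays the creature and provides a save point.
; A trigger overlap toggles its light and tracks whether the player-tagged creature is inside.
; Spray runs timed shower and water effects, calls InWater on the creature, then activates a linked door once and passes it to Camera_Tracker.
; SaveGame sets the creature's spawn and writes the spawn point location and current camera to BP_SaveGame.
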(event `Spray`
  (bind _doortoactivate_ (`self.DoorToActivate?`))
  (bind _shower (`self.Shower`))
  ;[1 1 1] Activate shower function
  (`ActorComponent.Activate` _shower false)
  (`ActorComponent.Activate` (`self.Water`) true)
  (bind _returnvalue (`GameplayStatics.GetActorOfClass` "/Game/Creature/CreatureCharacter.CreatureCharacter_C"))
  (`/Game/Creature/CreatureCharacter.InWater` _returnvalue)
  (`KismetSystemLibrary.Delay` 2.0)
  ;[1 1 1] activates any doors that are linked to the shower (if there are any)
  (`ActorComponent.Deactivate` _shower)
  (`ActorComponent.Deactivate` (`self.Water`))
  (if (`self.OneTimedoor`)
    (bind _asbp_door (cast `/Game/BluePrint/BP_Door` _doortoactivate_))
    (`/Game/BluePrint/BP_Door.IsActive` _asbp_door)
    (bind _returnvalue_2 (`GameplayStatics.GetActorOfClass` "/Game/BluePrint/Camera_Tracker.Camera_Tracker_C"))
    (set `/Game/BluePrint/Camera_Tracker.CurrentDoor` _doortoactivate_ _returnvalue_2)
    (set `self.OneTimedoor` false)))

(event `self.CreatureTrigger.OnComponentBeginOverlap`
  (params (OverlappedComponent :type "PrimitiveComponent Object Reference") (OtherActor :type "Actor Object Reference") (OtherComp :type "PrimitiveComponent Object Reference") (OtherBodyIndex :type Integer) (bFromSweep :type Boolean) (SweepResult :type "HitResult Structure (by ref)"))
  ;[1 1 1] Checks to see if the creature is currently in the shower hit box
  (set `self.IsInShower` (`self.ActorHasTag` OtherActor "Player"))
  (`SceneComponent.SetVisibility` (`self.PointLight`) true false))

(event `SaveGame`
  (bind _savegameref (`self.SaveGameRef`))
  ;[1 1 1] Save data to local file
  (bind _returnvalue (`GameplayStatics.GetActorOfClass` "/Game/Creature/CreatureCharacter.CreatureCharacter_C"))
  (`/Game/Creature/CreatureCharacter.SetCreatureSpawn` _returnvalue)
  (bind _returnvalue_2 (`GameplayStatics.DoesSaveGameExist` "SaveGame"))
  (if _returnvalue_2
    (bind _returnvalue_3 (`GameplayStatics.LoadGameFromSlot` "SaveGame"))
    (bind _asbp_save_game (cast `/Game/BluePrint/BP_SaveGame` _returnvalue_3))
    (set `self.SaveGameRef` _asbp_save_game)
    (else
      (bind _returnvalue_4 (`GameplayStatics.CreateSaveGameObject` "/Game/BluePrint/BP_SaveGame.BP_SaveGame_C"))
      (bind _output_get (set `self.SaveGameRef` _returnvalue_4))))
  (bind _returnvalue_5 (`GameplayStatics.GetActorOfClass` "/Game/Creature/CreatureCharacter.CreatureCharacter_C"))
  (set `/Game/BluePrint/BP_SaveGame.CreatureLocation` (`self.K2_GetActorLocation` (`self.SpawnPoint`)) _output_get)
  (set `/Game/BluePrint/BP_SaveGame.CameraIndex` (`/Game/Creature/CreatureCharacter.CurrentCamera` _returnvalue_5) _savegameref)
  (bind _returnvalue_6 (`GameplayStatics.SaveGameToSlot` _savegameref "SaveGame"))
  (if _returnvalue_6
    (`KismetSystemLibrary.PrintString` "SaveGameSuccessfully")
    (else
      (`KismetSystemLibrary.PrintString` "FailedToSaveGame"))))

(event `self.CreatureTrigger.OnComponentEndOverlap`
  (params (OverlappedComponent :type "PrimitiveComponent Object Reference") (OtherActor :type "Actor Object Reference") (OtherComp :type "PrimitiveComponent Object Reference") (OtherBodyIndex :type Integer))
  ;[1 1 1] Checks to see if the creature is currently in the shower hit box
  (set `self.IsInShower` false)
  (`SceneComponent.SetVisibility` (`self.PointLight`) false false))

(fn `UserConstructionScript`)