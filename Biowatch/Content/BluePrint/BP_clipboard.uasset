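; Clickable clipboard actor that plays an animation forward and in reverse on alternating clicks.
; BeginPlay enables click events, creates a player for the ClipBoardAnimation level sequence, and makes dynamic materials for the board and paper.
; Each click plays the Clipboard component and flip-flops the sequence direction, with forward clicks also stopping the flash.
; StartFlash and StopFlash drive the flashspeed parameter on both materials to toggle a flashing highlight.
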(event `self.ReceiveBeginPlay`
  (set `PlayerController.bEnableClickEvents` true (`GameplayStatics.GetPlayerController` 0))
  (bind (_outactor _returnvalue) (`LevelSequencePlayer.CreateLevelSequencePlayer` "/Game/BluePrint/ClipBoardAnimation.ClipBoardAnimation" (`self.Settings`)))
  (bind _returnvalue_2 (`PrimitiveComponent.CreateDynamicMaterialInstance` (`self.Board`) 0 "/Game/BluePrint/Import/M_clipboardWood.M_clipboardWood" "None"))
  (set `self.WoodFlash` _returnvalue_2)
  (bind _returnvalue_3 (`PrimitiveComponent.CreateDynamicMaterialInstance` (`self.paper`) 0 null "None"))
  (set `self.Paperflash` _returnvalue_3))

(event `self.ReceiveActorOnClicked`
  (params (ButtonPressed :type "Key Structure"))
  (`AudioComponent.Play` (`self.Clipboard`) 0.0)
  (`/Engine/EditorBlueprintResources/StandardMacros.FlipFlop`
    (:`A`
      (`self.StopFlash`)
      (`MovieSceneSequencePlayer.Play` (stale `self.ReceiveBeginPlay` _returnvalue)))
    (:`B`
      (`MovieSceneSequencePlayer.PlayReverse` (stale `self.ReceiveBeginPlay` _returnvalue)))))

(event `StopFlash`
  (`MaterialInstanceDynamic.SetScalarParameterValue` (`self.WoodFlash`) "flashspeed" 0.0)
  (`MaterialInstanceDynamic.SetScalarParameterValue` (`self.Paperflash`) "flashspeed" 0.0))

(event `StartFlash`
  (`MaterialInstanceDynamic.SetScalarParameterValue` (`self.WoodFlash`) "flashspeed" 0.4)
  (`MaterialInstanceDynamic.SetScalarParameterValue` (`self.Paperflash`) "flashspeed" 0.4))

(fn `UserConstructionScript`)