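; Sliding door Blueprint that moves vertically between open and closed positions, with an indicator light.
; ToggleDoor flips IsOpen and uses MoveComponentTo to animate the Door component down to open or up to close over a fixed duration.
; BeginPlay opens the door when StartOpen is set.
; IsActive and IsInactive events switch PointLight1 between green and red.
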(event `self.ReceiveBeginPlay`
  (if (`self.StartOpen?`)
    (set `self.IsOpen?` true :!label _label)
    (`KismetSystemLibrary.MoveComponentTo` (`self.Door`) (0.0 0.0 -350.0) (struct :`Yaw` 90.0) false false 2.0)))

(event `Toggle Door`
  (if (`self.IsOpen?`)
    (set `self.IsOpen?` false)
    (`KismetSystemLibrary.MoveComponentTo` (`self.Door`) (0.0 0.0 130.0) (struct :`Yaw` 90.0) false false 2.0)
    (else
      (goto _label))))

(event `IsActive`
  (`LightComponent.SetLightColor` (`self.PointLight1`) (struct :`R` 0.351989 :`G` 1.0 :`A` 1.0) true))

(event `IsInactive`
  (`LightComponent.SetLightColor` (`self.PointLight1`) (struct :`R` 1.0 :`B` 0.037799 :`A` 1.0) true))

(fn `UserConstructionScript`)