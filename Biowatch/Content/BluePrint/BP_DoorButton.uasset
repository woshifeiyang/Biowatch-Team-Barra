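; BP_DoorButton is a clickable button actor that toggles the current door.
; BeginPlay enables click events on the first player controller.
; A click plays the OfficeButton sound and animates the Button component downward with MoveComponentTo.
; It then finds the Camera_Tracker actor by class, calls ToggleCurrentDoor on it, which decides the door, and moves the button back.
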(event `self.ReceiveBeginPlay`
  (set `PlayerController.bEnableClickEvents` true (`GameplayStatics.GetPlayerController` 0)))

(event `self.ReceiveActorOnClicked`
  (params (ButtonPressed :type "Key Structure"))
  (`AudioComponent.Play` (`self.OfficeButton`) 0.0)
  (`KismetSystemLibrary.MoveComponentTo` (`self.Button`) (0.0 0.0 -8.0) (struct) false false 0.25)
  (bind _returnvalue (`GameplayStatics.GetActorOfClass` "/Game/BluePrint/Camera_Tracker.Camera_Tracker_C"))
  (`/Game/BluePrint/Camera_Tracker.ToggleCurrentDoor` _returnvalue)
  (`KismetSystemLibrary.MoveComponentTo` (`self.Button`) (0.0 0.0 0.0) (struct) false false 0.25))

(fn `UserConstructionScript`)