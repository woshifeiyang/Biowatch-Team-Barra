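; Camera_Tracker is the player's surveillance controller, possessing level cameras, cycling between them and toggling to an office view with a camera UI.
; Right-click fires the current camera's laser once the pod is open and spawns a target under the cursor, which the living creature moves toward via AI if a line trace finds it visible.
; Release or camera switching stops the creature.
; Events toggle doors and open the pod; the looping laser timer event is an empty stub.
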(event `self.ReceiveBeginPlay`
  (bind _returnvalue (`GameplayStatics.GetPlayerController` 0))
  (bind _cameras (`self.Cameras`))
  (bind _output (`|GetArrayItem` _cameras (`self.current cam`)))
  ;[1 1 1] Makes player possess first camera in level / enables the actor to accept player input / enables mouse visability / Display Camera UI
  (set `PlayerController.bShowMouseCursor` true _returnvalue)
  (`self.EnableInput` _returnvalue)
  (set `self.Number of cams` (- (`KismetArrayLibrary.Array_Length` _cameras) 1))
  (`Controller.Possess` _returnvalue _output)
  (bind _ascamera (cast `/Game/BluePrint/Camera` _output))
  (`/Game/BluePrint/Camera.SetScreen` _ascamera)
  (`self.EnableInput` _returnvalue)
  (bind _returnvalue_2 (`|CreateWidget` "/Game/BluePrint/WB_CameraView.WB_CameraView_C" null null))
  (bind _output_get (set `self.CameraUIWidget` _returnvalue_2))
  (`UserWidget.AddToViewport` _output_get 0))

(event `InputAction|SwitchRightCamera`
  (params (Key :type "Key Structure"))
  (bind _current_cam (`self.current cam`))
  ;[1 1 1] D button adds 1 onto the current camera value and then posses the camera with the value equal to the new number
  (:`Pressed`
    (if (not (`self.InOffice?`))
      (bind _ascamera (cast `/Game/BluePrint/Camera` (`|GetArrayItem` (`self.Cameras`) _current_cam)))
      (`/Game/BluePrint/Camera.UnsetScreen` _ascamera)
      (bind _result (`/Engine/EditorBlueprintResources/StandardMacros.IncrementInt` _current_cam)
        (:`  `
          (bind _output_get (set `self.current cam` (`KismetMathLibrary.Clamp` _result 0 (`self.Number of cams`))))
          (bind _output (`|GetArrayItem` (`self.Cameras`) _output_get))
          (`Controller.Possess` (`GameplayStatics.GetPlayerController` 0) _output)
          (bind _ascamera_2 (cast `/Game/BluePrint/Camera` _output))
          (`/Game/BluePrint/Camera.SetScreen` _ascamera_2)
          (`KismetSystemLibrary.PrintString` (`KismetStringLibrary.Conv_IntToString` (`self.current cam`)))
          (`/Game/BluePrint/Camera.endlaser` _ascamera)
          (`self.StopCreature`))))))

(event `InputAction|SwitchLeftCamera`
  (params (Key :type "Key Structure"))
  (bind _current_cam (`self.current cam`))
  ;[1 1 1] A button takes away 1 from the current camera number and then posses the camera with the number value equal to the new number
  (:`Pressed`
    (if (not (`self.InOffice?`))
      (bind _ascamera (cast `/Game/BluePrint/Camera` (`|GetArrayItem` (`self.Cameras`) _current_cam)))
      (`/Game/BluePrint/Camera.UnsetScreen` _ascamera)
      (bind _result (`/Engine/EditorBlueprintResources/StandardMacros.DecrementInt` _current_cam)
        (:`  `
          (bind _output_get (set `self.current cam` (`KismetMathLibrary.Clamp` _result 0 (`self.Number of cams`))))
          (bind _output (`|GetArrayItem` (`self.Cameras`) _output_get))
          (`Controller.Possess` (`GameplayStatics.GetPlayerController` 0) _output)
          (bind _ascamera_2 (cast `/Game/BluePrint/Camera` _output))
          (`/Game/BluePrint/Camera.SetScreen` _ascamera_2)
          (`KismetSystemLibrary.PrintString` (`KismetStringLibrary.Conv_IntToString` (`self.current cam`)))
          (`/Game/BluePrint/Camera.endlaser` _ascamera)
          (`self.StopCreature`))))))

(event `LaserFIre`
  ;[1 1 1] (WIP) Laser fire
)

(event `StopCreature`
  ;[1 1 1] Stops creature movment when called
  (bind _returnvalue (`GameplayStatics.GetActorOfClass` "/Game/Creature/CreatureCharacter.CreatureCharacter_C"))
  (`Controller.StopMovement` (`Pawn.GetController` _returnvalue)))

(event `InputAction|RightMouseClick`
  (params (Key :type "Key Structure"))
  ;[1 1 1] Right click stops moving camera on press and starts again on release
  (:`Pressed`
    (bind _output (`|GetArrayItem` (`self.Cameras`) (stale `InputAction|SwitchLeftCamera` _output_get)))
    (bind _ascamera (cast `/Game/BluePrint/Camera` _output))
    ;[1 1 1] Checks to see if you should be able to use the laser/ stops the laser and creature
    (if (`self.InOffice?`)
      _
      (elif (`self.PodOpen`)
        (bind _returnvalue (`GameplayStatics.GetActorOfClass` "/Game/Creature/CreatureCharacter.CreatureCharacter_C"))
        (if (not (`/Game/Creature/CreatureCharacter.IsDead` _returnvalue))
          (`/Game/BluePrint/Camera.firelaser` _ascamera)
          ;[1 1 1] Sets a looping timer that moves the creature to the clicked location and stops when no longer holding the click
          (bind _returnvalue_2 (`KismetSystemLibrary.K2_SetTimerDelegate` (delegate `LaserFIre`) 0.1 true))
          (bind _returnvalue_3 (`|SpawnActorFromClass` "/Game/BluePrint/BP_creatureTarget.BP_creatureTarget_C" (`KismetMathLibrary.MakeTransform` (`.ImpactPoint` (`GameplayStatics.BreakHitResult` (`PlayerController.GetHitResultUnderCursorByChannel` (`GameplayStatics.GetPlayerController` 0) "TraceTypeQuery1" true))) (struct) (0.5 0.5 0.5)) "Undefined" "OverrideRootScale" null null))
          (`/Engine/EditorBlueprintResources/StandardMacros.IsValid` _returnvalue_3
            (:`Is Valid`
              (set `Actor.Tags` (`|MakeArray` "TargetPoint" :!type "Name") _returnvalue_3)
              (`KismetSystemLibrary.PrintString` "CreatActorSuccessfully")
              (bind _output_get (set `self.TargetPoint` _returnvalue_3))
              (`self.CanCreatureSee`)
              (if (`self.CreatureVision`)
                (`AIController.MoveToActor` (`AIBlueprintHelperLibrary.GetAIController` _returnvalue) _output_get -1.0 true true false null true)))
            (:`Is Not Valid`
              (`KismetSystemLibrary.PrintString` "TargetPoint is null")))))))
  (:`Released`
    (bind _ascamera_2 (cast `/Game/BluePrint/Camera` _output))
    (`/Game/BluePrint/Camera.endlaser` _ascamera_2)
    (`self.StopCreature`)
    (`KismetSystemLibrary.K2_InvalidateTimerHandle` _returnvalue_2)
    (`self.K2_DestroyActor` _output_get)))

(event `ToggleCurrentDoor`
  ;[1 1 1] Opens/closes the current door
  (bind _asbp_door (cast `/Game/BluePrint/BP_Door` (`self.CurrentDoor`)))
  (`/Game/BluePrint/BP_Door.Toggle Door` _asbp_door))

(event `PodIsopen`
  ;[1 1 1] set the pod to open
  (set `self.PodOpen` true))

(event `Key|W`
  (params (Key :type "Key Structure"))
  (bind _returnvalue (`GameplayStatics.GetPlayerController` 0))
  ;[1 1 1] Toggle from current cam to office view
  (:`Pressed`
    (if (`self.InOffice?`)
      (`Controller.Possess` _returnvalue (`|GetArrayItem` (`self.Cameras`) (`self.current cam`)))
      (`self.EnableInput` null)
      (bind _returnvalue_2 (`|CreateWidget` "/Game/BluePrint/WB_CameraView.WB_CameraView_C" null null))
      (bind _output_get (set `self.CameraUIWidget` _returnvalue_2))
      (`UserWidget.AddToViewport` _output_get 0)
      (set `self.InOffice?` false)
      (else
        (`Widget.RemoveFromParent` (`self.CameraUIWidget`))
        (`Controller.Possess` _returnvalue (`self.Office_cam`))
        (`KismetSystemLibrary.PrintString` "Office")
        (set `self.InOffice?` true)))))

(event `CanCreatureSee`
  ;[1 1 1] Checks to see if the creature can see the laser point from its current possition
  (bind _returnvalue (`GameplayStatics.GetActorOfClass` "/Game/Creature/CreatureCharacter.CreatureCharacter_C"))
  (bind (_outhit _returnvalue_2) (`KismetSystemLibrary.LineTraceSingle` :`Start` (`SceneComponent.K2_GetComponentLocation` (`Character.CapsuleComponent` _returnvalue)) :`End` (`.ImpactPoint` (`GameplayStatics.BreakHitResult` (`PlayerController.GetHitResultUnderCursorByChannel` (`GameplayStatics.GetPlayerController` 0) "TraceTypeQuery1" true))) :`TraceChannel` "TraceTypeQuery1" :`DrawDebugType` "Persistent"))
  (if _returnvalue_2
    (if (`ActorComponent.ComponentHasTag` (`.HitComponent` (`GameplayStatics.BreakHitResult` _outhit)) "LaserPoint")
      (set `self.CreatureVision` true :!label _label)
      (else
        (set `self.CreatureVision` false)))
    (else
      (goto _label))))

(fn `UserConstructionScript`)